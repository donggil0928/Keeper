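; Scythe projectile for a W skill that spins and, when CanReturn is set, flies back like a boomerang.
; Tick rotates the pivot, flags the return once MaxDistance from spawn is reached, then re-aims at the KeeperCharacter each frame in 2D.
; While returning, overlaps apply a force pulling MonsterBase actors toward the Keeper, and touching the Keeper destroys the projectile.
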(event `self.ReceiveBeginPlay`)

(event `self.ReceiveTick`
  (params (DeltaSeconds :type "Float (single-precision)"))
  (`SceneComponent.K2_AddLocalRotation` (`self.ProjectilePivot`) (`KismetMathLibrary.MakeRotator` 0.0 (* DeltaSeconds (`self.RotationSpeed`))) false false)
  (if (`self.bCanReturn`)
    (if (not (`self.bIsReturn`))
      (bind _output_get (set `self.CurrentDistance` (`KismetMathLibrary.Vector_Distance` (`self.SpawnedLocation`) (`self.K2_GetActorLocation`))))
      (if (>= _output_get (`self.MaxDistance`))
        (set `self.bIsReturn` true))
      (else
        (bind _returnvalue (`GameplayStatics.GetActorOfClass` "/Script/Keeper.KeeperCharacter"))
        (`self.FireInDirection` (`KismetMathLibrary.Vector_Normal2D` (- (`self.K2_GetActorLocation` _returnvalue) (`self.K2_GetActorLocation`))))))))

(event `self.ReceiveActorBeginOverlap`
  (params (OtherActor :type "Actor Object Reference"))
  (if (`self.bIsReturn`)
    (if (and (`KismetSystemLibrary.IsValid` OtherActor) (!= OtherActor self))
      (`|ExecutionSequence`
        (:`then_0`
          (bind _asmonster_base (cast `MonsterBase` OtherActor))
          (if (`KismetSystemLibrary.IsValid` _asmonster_base)
            (set `self.GrabDirection` (`self.GetActorForwardVector` _asmonster_base))
            (`|ExecutionSequence`
              (:`then_0`
                (bind _returnvalue (`GameplayStatics.GetActorOfClass` "/Script/Keeper.KeeperCharacter"))
                (if (`KismetSystemLibrary.IsValid` _returnvalue)
                  (set `self.GrabDirection` (`KismetMathLibrary.Vector_Normal2D` (- (`self.K2_GetActorLocation` _returnvalue) (`self.K2_GetActorLocation` _asmonster_base))))))
              (:`then_1`
                (`CharacterMovementComponent.AddForce` (`Character.CharacterMovement` _asmonster_base) (* (`self.GrabDirection`) (`self.GrabPower`)))))))
        (:`then_1`
          (bind _askeeper_character (cast `KeeperCharacter` OtherActor))
          (if (`KismetSystemLibrary.IsValid` _askeeper_character)
            (`self.DestroyProjectile`)))))))

(fn `UserConstructionScript`)