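; Skill effect actor that turns a target KeeperCharacter into a sub-shooter for the Default R skill and gives it a small heal.
; On activation it binds ShootTheMonster to the keeper's sub-shooter delegate and adds HP, clamped to MaxHP.
; Each delegate call spawns a BP_Default_R at the keeper's transform with a spherical damage field and limited lifespan.
; Destruction unbinds all events from that delegate, not just its own.
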(event `self.ActivateEffectImplement`
  (bind _askeeper_character (cast `KeeperCharacter` (`self.Target`)))
  (add `KeeperCharacter.SubShooterDelegate` _askeeper_character (delegate `ShootTheMonster`))
  (set `KeeperCharacter.CurrentHP` (`KismetMathLibrary.Clamp` (+ (`KeeperCharacter.CurrentHP` _askeeper_character) 20) 0 (`KeeperCharacter.MaxHP` _askeeper_character)) _askeeper_character))

(event `ShootTheMonster`
  (bind (_returnvalue_location _returnvalue_rotation) (`KismetMathLibrary.BreakTransform` (`self.GetTransform` (`self.Target`))))
  (bind _returnvalue (`|SpawnActorFromClass` "/Game/Blueprints/TempSkill/BP_Default_R.BP_Default_R_C" (`KismetMathLibrary.MakeTransform` _returnvalue_location _returnvalue_rotation) "AdjustIfPossibleButAlwaysSpawn" "MultiplyWithRoot" null null))
  (`DamageField_Base.CreateDamageField_Sphere` _returnvalue 100.0)
  (`self.SetLifeSpan` _returnvalue (`self.DamageFieldLifeTime`)))

(event `self.ReceiveDestroyed`
  (bind _askeeper_character (cast `KeeperCharacter` (`self.Target`)))
  (clear `KeeperCharacter.SubShooterDelegate` _askeeper_character))

(fn `UserConstructionScript`)