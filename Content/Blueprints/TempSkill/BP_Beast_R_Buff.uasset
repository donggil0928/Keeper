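; Beast R skill buff that temporarily boosts a KeeperCharacter target's attack power and damage radius.
; On effect activation it caches both current values, then raises attack power to 3.5 times (truncated) and radius to 2.5 times.
; When the buff actor is destroyed it writes the cached values back, overwriting any changes made to those stats meanwhile.
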(event `self.ActivateEffectImplement`
  (bind _askeeper_character (cast `KeeperCharacter` (`self.Target`)))
  (`|ExecutionSequence`
    (:`then_0`
      (bind _output_get (set `self.PrevAttackPower` (`KeeperCharacter.AttackPower` _askeeper_character)))
      (set `KeeperCharacter.AttackPower` (`KismetMathLibrary.FTrunc` (+ _output_get (* _output_get 2.5))) _askeeper_character))
    (:`then_1`
      (bind _output_get_2 (set `self.PrevDamageRadius` (`KeeperCharacter.DamageRadius` _askeeper_character)))
      (set `KeeperCharacter.DamageRadius` (* _output_get_2 2.5) _askeeper_character))))

(event `self.ReceiveDestroyed`
  (bind _askeeper_character (cast `KeeperCharacter` (`self.Target`)))
  (`|ExecutionSequence`
    (:`then_0`
      (set `KeeperCharacter.AttackPower` (`self.PrevAttackPower`) _askeeper_character))
    (:`then_1`
      (set `KeeperCharacter.DamageRadius` (`self.PrevDamageRadius`) _askeeper_character))))

(fn `UserConstructionScript`)