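; BP_Beast_E is a skill effect that lowers the defence of nearby monsters.
; On activation, a sphere overlap of radius ReduceRange on WorldStatic objects finds MonsterBase actors, stores each one and its MonsterDef, then subtracts a fixed amount.
; On destruction it rewrites each monster's defence using Find on the saved values with the loop index, which searches by value instead of reading that slot.
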(event `self.ActivateEffectImplement`
  (bind _outactors (`KismetSystemLibrary.SphereOverlapActors` (0.0 0.0 0.0) (`self.ReduceRange`) (`|MakeArray` (enumliteral `EObjectTypeQuery` "ObjectTypeQuery1")) "/Script/Keeper.MonsterBase" (`|MakeArray` (`self.Target`))))
  (for _array_element _outactors
    (bind _asmonster_base (cast `MonsterBase` _array_element))
    (`KismetArrayLibrary.Array_Add` (`self.Monsters`) _asmonster_base)
    (bind _monsterdef (`MonsterBase.MonsterDef` _asmonster_base))
    (`KismetArrayLibrary.Array_Add` (`self.PrevDefenceNums`) _monsterdef)
    (set `MonsterBase.MonsterDef` (- _monsterdef 10) _asmonster_base)))

(event `self.ReceiveDestroyed`
  (for (_array_element _array_index) (`self.Monsters`)
    (bind _asmonster_base (cast `MonsterBase` _array_element))
    (set `MonsterBase.MonsterDef` (`KismetArrayLibrary.Array_Find` (`self.PrevDefenceNums`) _array_index) _asmonster_base)))

(fn `UserConstructionScript`)