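; BP_PlayCutScene is a trigger actor that plays a level sequence cutscene once, when any actor first overlaps it.
; The overlap sets a HasPlayed flag, calls DisableInput, stops the first player controller's movement and starts a sequence player created for the CutScene asset.
; The sequence's OnFinished event calls EnableInput to return control when playback ends.
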(event `self.ReceiveActorBeginOverlap`
  (params (OtherActor :type "Actor Object Reference"))
  (bind _returnvalue (`GameplayStatics.GetPlayerController` 0))
  (if (not (`self.bHasPlayed`))
    (set `self.bHasPlayed` true)
    (`self.DisableInput` _returnvalue)
    (`Controller.StopMovement` _returnvalue)
    (bind (_outactor _returnvalue_2) (`LevelSequencePlayer.CreateLevelSequencePlayer` "/Game/CutScene/CutScene.CutScene"))
    (`MovieSceneSequencePlayer.Play` _returnvalue_2)
    (add `MovieSceneSequencePlayer.OnFinished` _returnvalue_2 (delegate `On Sequence Finished`))))

(event `On Sequence Finished`
  (`self.EnableInput` (`GameplayStatics.GetPlayerController` 0) null))

(fn `UserConstructionScript`)